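; BP_Pickup is a pickup actor that shows an animated outline while the player character is near it, with no collection logic yet.
; On BeginPlay it replaces the static mesh's overlay material with a dynamic instance.
; Sphere overlaps with BP_ThirdPersonCharacter trigger InRange and OutOfRange, which play or reverse the LerpOutline timeline to animate the material's LineThickness parameter.
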(event `self.ReceiveBeginPlay`
  (bind _returnvalue (`KismetMaterialLibrary.CreateDynamicMaterialInstance` (`MeshComponent.GetOverlayMaterial` (`self.StaticMesh`))))
  (bind _output_get (set `self.DynamicMaterial` _returnvalue))
  (`MeshComponent.SetOverlayMaterial` (`self.StaticMesh`) _output_get))

(event `self.Sphere.OnComponentBeginOverlap`
  (params (OverlappedComponent :type "PrimitiveComponent Object Reference") (OtherActor :type "Actor Object Reference") (OtherComp :type "PrimitiveComponent Object Reference") (OtherBodyIndex :type Integer) (bFromSweep :type Boolean) (SweepResult :type "HitResult Structure (by ref)"))
  (cast `/Game/ThirdPerson/Blueprints/BP_ThirdPersonCharacter` OtherActor)
  (`self.InRange`))

(event `self.Sphere.OnComponentEndOverlap`
  (params (OverlappedComponent :type "PrimitiveComponent Object Reference") (OtherActor :type "Actor Object Reference") (OtherComp :type "PrimitiveComponent Object Reference") (OtherBodyIndex :type Integer))
  (cast `/Game/ThirdPerson/Blueprints/BP_ThirdPersonCharacter` OtherActor)
  (`self.OutOfRange`))

(event `InRange`
  (`|ExecutionSequence`
    (:`then_0`
      (bind (_direction _alpha) (`Timeline|LerpOutline` :!via `Stop` :!label _label)
        (:`Update`
          (`MaterialInstanceDynamic.SetScalarParameterValue` (`self.DynamicMaterial`) "LineThickness" _alpha))))
    (:`then_1`
      (goto _label))))

(event `OutOfRange`
  (`|ExecutionSequence`
    (:`then_0`
      (goto _label :!via `Stop`))
    (:`then_1`
      (goto _label :!via `Reverse`))))

(fn `UserConstructionScript`)