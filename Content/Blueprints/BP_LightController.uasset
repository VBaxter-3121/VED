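; BP_LightController is an interactable that moves linked light groups left or right.
; Its sphere overlap registers it with BP_ThirdPersonCharacter, toggles instructions and lerps each group's child lights in or out, also drawing debug traces to each group on entry.
; Tick moves every group while a direction flag is set.
; ChangeIndex cycles a selected group index with wraparound, but movement ignores it because the selection checks are disconnected.
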(event `self.ReceiveBeginPlay`)

(event `self.ReceiveTick`
  (params (DeltaSeconds :type "Float (single-precision)"))
  (if (`self.MoveLightsRight`)
    (`self.Move Lights Right`)
    (elif (`self.MoveLightsLeft`)
      (`self.Move Lights Left`))))

(event `self.Sphere.OnComponentBeginOverlap`
  (params (OverlappedComponent :type "PrimitiveComponent Object Reference") (OtherActor :type "Actor Object Reference") (OtherComp :type "PrimitiveComponent Object Reference") (OtherBodyIndex :type Integer) (bFromSweep :type Boolean) (SweepResult :type "HitResult Structure (by ref)"))
  (bind _asbp_third_person_character (cast `/Game/ThirdPerson/Blueprints/BP_ThirdPersonCharacter` OtherActor))
  (set `/Game/ThirdPerson/Blueprints/BP_ThirdPersonCharacter.LightControllerInRange` true _asbp_third_person_character)
  (`SceneComponent.SetVisibility` (`self.Instructions`) true false)
  (`/Game/ThirdPerson/Blueprints/BP_ThirdPersonCharacter.SetLightController` _asbp_third_person_character self)
  (for _array_element (`self.LightGroups`)
    (bind _outactors (`GameplayStatics.GetAllActorsOfClass` "/Game/ThirdPerson/Blueprints/BP_ThirdPersonCharacter.BP_ThirdPersonCharacter_C"))
    (`KismetSystemLibrary.LineTraceSingleByProfile` (`self.K2_GetActorLocation`) (`self.K2_GetActorLocation` _array_element) "None" false _outactors "ForDuration" true (struct :`G` 1.0 :`A` 1.0))
    (for _array_element_2 (`/Game/Blueprints/BP_LightGroup.ChildLights` _array_element)
      (`/Game/Blueprints/BP_LightStrip.LerpIn` _array_element_2))))

(event `self.Sphere.OnComponentEndOverlap`
  (params (OverlappedComponent :type "PrimitiveComponent Object Reference") (OtherActor :type "Actor Object Reference") (OtherComp :type "PrimitiveComponent Object Reference") (OtherBodyIndex :type Integer))
  (bind _asbp_third_person_character (cast `/Game/ThirdPerson/Blueprints/BP_ThirdPersonCharacter` OtherActor))
  (set `/Game/ThirdPerson/Blueprints/BP_ThirdPersonCharacter.LightControllerInRange` false _asbp_third_person_character)
  (`SceneComponent.SetVisibility` (`self.Instructions`) false false)
  (for _array_element (`self.LightGroups`)
    (for _array_element_2 (`/Game/Blueprints/BP_LightGroup.ChildLights` _array_element)
      (`/Game/Blueprints/BP_LightStrip.LerpOut` _array_element_2))))

(event `Change Index`
  (params (Increment :type Integer))
  (bind _returnvalue (`KismetArrayLibrary.Array_Length` (`self.LightGroups`)))
  (bind _returnvalue_2 (+ Increment (`self.SelectedLightGroupIndex`)))
  (if (< _returnvalue_2 _returnvalue)
    (if (>= _returnvalue_2 0)
      (set `self.SelectedLightGroupIndex` _returnvalue_2)
      (else
        (set `self.SelectedLightGroupIndex` (- _returnvalue 1))))
    (else
      (set `self.SelectedLightGroupIndex` 0))))

(event `Move Lights Right`
  (for (_array_element _array_index) (`self.LightGroups`)
    (`/Game/Blueprints/BP_LightGroup.MoveGroup` _array_element 1)))

(event `Move Lights Left`
  (for (_array_element _array_index) (`self.LightGroups`)
    (`/Game/Blueprints/BP_LightGroup.MoveGroup` _array_element -1)))

(fn `UserConstructionScript`)