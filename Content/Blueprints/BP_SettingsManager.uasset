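; BP_SettingsManager loads player settings from a save slot and applies the master volume.
; Init reads Volume, Brightness and Sensitivity from an existing BP_SettingsSave, or creates and saves a new one, keeping the manager's own values.
; Apply sets a sound class override on the master mix, then pushes that mix after a short delay.
; Brightness and Sensitivity are not applied here.
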(event `self.ReceiveInit`
  (bind _returnvalue (`GameplayStatics.DoesSaveGameExist` "SettingsSlot"))
  (if _returnvalue
    (bind _returnvalue_2 (`GameplayStatics.LoadGameFromSlot` "SettingsSlot"))
    (bind _asbp_settings_save (cast `/Game/Blueprints/BP_SettingsSave` _returnvalue_2))
    (bind _output_get (set `self.SettingsSave` _asbp_settings_save))
    (`/Engine/EditorBlueprintResources/StandardMacros.IsValid` _output_get
      (:`Is Valid`
        (set `self.Volume` (`/Game/Blueprints/BP_SettingsSave.Volume` _output_get))
        (set `self.Brightness` (`/Game/Blueprints/BP_SettingsSave.Brightness` _output_get))
        (set `self.Sensitivity` (`/Game/Blueprints/BP_SettingsSave.Sensitivity` _output_get))))
    (else
      (bind _returnvalue_3 (`GameplayStatics.CreateSaveGameObject` "/Game/Blueprints/BP_SettingsSave.BP_SettingsSave_C"))
      (bind _output_get_2 (set `self.SettingsSave` _returnvalue_3))
      (`GameplayStatics.SaveGameToSlot` _output_get_2 "SettingsSlot")))
  (`self.Apply`))

(event `Apply`
  (`GameplayStatics.SetSoundMixClassOverride` "/Game/Blueprints/SCM_MasterMix.SCM_MasterMix" "/Game/Blueprints/SC_Master.SC_Master" (`self.Volume`))
  (`KismetSystemLibrary.Delay` 0.2)
  (`GameplayStatics.PushSoundMixModifier` "/Game/Blueprints/SCM_MasterMix.SCM_MasterMix"))