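; Enemy character Blueprint that sets its walk speed on spawn and handles its own death through a Kill event.
; Kill stops movement, plays a random death animation and swaps two mesh material slots to M_Invisible.
; A dynamic instance of that material becomes the mesh overlay, with FadeTimeline driving its Opacity until the actor is destroyed when the timeline finishes.
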(event `self.ReceiveBeginPlay`
  (set `CharacterMovementComponent.MaxWalkSpeed` 300.0 (`self.CharacterMovement`)))

(event `Kill`
  (set `CharacterMovementComponent.MaxWalkSpeed` 0.0 (`self.CharacterMovement`))
  (bind _returnvalue (`KismetMaterialLibrary.CreateDynamicMaterialInstance` "/Game/Materials/M_Invisible.M_Invisible"))
  (bind _output_get (set `self.FadeMaterial` _returnvalue))
  (`MaterialInstanceDynamic.SetScalarParameterValue` _output_get "Opacity" 1.0)
  (`PrimitiveComponent.SetMaterial` (`self.Mesh`) 0 "/Game/Materials/M_Invisible.M_Invisible")
  (`PrimitiveComponent.SetMaterial` (`self.Mesh`) 1 "/Game/Materials/M_Invisible.M_Invisible")
  (`MeshComponent.SetOverlayMaterial` (`self.Mesh`) (`self.FadeMaterial`))
  (`SkeletalMeshComponent.PlayAnimation` (`self.Mesh`) (`KismetArrayLibrary.Array_Random` (`self.DeathAnims`)) false)
  (bind (_direction _alpha) (`Timeline|FadeTimeline` :!via `PlayFromStart`)
    (:`Update`
      (`MaterialInstanceDynamic.SetScalarParameterValue` (`self.FadeMaterial`) "Opacity" _alpha))
    (:`Finished`
      (`self.K2_DestroyActor`))))

(fn `UserConstructionScript`)