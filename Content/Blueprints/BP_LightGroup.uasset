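; BP_LightGroup is an actor that slides itself and a set of child light actors along the world Y axis.
; BeginPlay stores each light's Y offset as group Y minus light Y.
; MoveGroup steps by MoveSpeed in the given Direction within YMin/YMax checks, then repositions every light at the group's X and Z.
; Each stored offset is added to group Y, which mirrors the lights' original layout around the group.
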(event `self.ReceiveBeginPlay`
  (bind (_returnvalue_x _returnvalue_y) (`KismetMathLibrary.BreakVector` (`self.K2_GetActorLocation`)))
  (for _array_element (`self.ChildLights`)
    (bind (_returnvalue_x_2 _returnvalue_y_2) (`KismetMathLibrary.BreakVector` (`self.K2_GetActorLocation` _array_element)))
    (`KismetArrayLibrary.Array_Add` (`self.YOffsets`) (- _returnvalue_y _returnvalue_y_2))))

(event `MoveGroup`
  (params (Direction :type Integer))
  (bind (_returnvalue_x _returnvalue_y _returnvalue_z) (`KismetMathLibrary.BreakVector` (`self.K2_GetActorLocation`)))
  (bind (_returnvalue_x_2 _returnvalue_y_2 _returnvalue_z_2) (`KismetMathLibrary.BreakVector` (`self.K2_GetActorLocation`)))
  (bind _output_get (set `self.Direction` Direction))
  (if (or (and (== _output_get 1) (< _returnvalue_y (`self.YMax`))) (and (== _output_get -1) (> _returnvalue_y (`self.YMin`))))
    (`self.K2_SetActorLocation` (`KismetMathLibrary.MakeVector` _returnvalue_x (+ (* (`self.MoveSpeed`) Direction) _returnvalue_y) _returnvalue_z))
    (for (_array_element _array_index) (`self.ChildLights`)
      (`self.K2_SetActorLocation` _array_element (`KismetMathLibrary.MakeVector` _returnvalue_x_2 (+ _returnvalue_y_2 (`|GetArrayItem` (`self.YOffsets`) _array_index)) _returnvalue_z_2) false false))))

(fn `UserConstructionScript`)