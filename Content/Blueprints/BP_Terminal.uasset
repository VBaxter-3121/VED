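; BP_Terminal is an interactable terminal that needs a power cell and drives a linked puzzle widget.
; Entering its sphere with a carried cell consumes it and powers the terminal, which then registers itself with the character while the prompt shows power status.
; BeginPlay links the terminal to the final puzzle widget.
; Its Complete event plays sounds and music, lights the linked lights and triggers the linked spawns.
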(event `self.ReceiveBeginPlay`
  (bind _aswbp_pickup (cast `/Game/UI/WBP_Pickup` (`WidgetComponent.GetUserWidgetObject` (`self.Widget`))))
  (`/Game/UI/WBP_Pickup.Set Text` _aswbp_pickup "NO POWER")
  (bind _aswbp_terminal_puzzle_final (cast `/Game/UI/WBP_TerminalPuzzleFinal` (`self.Puzzle`)))
  (`/Game/UI/WBP_TerminalPuzzleFinal.LinkTerminal` _aswbp_terminal_puzzle_final self))

(event `self.Sphere.OnComponentBeginOverlap`
  (params (OverlappedComponent :type "PrimitiveComponent Object Reference") (OtherActor :type "Actor Object Reference") (OtherComp :type "PrimitiveComponent Object Reference") (OtherBodyIndex :type Integer) (bFromSweep :type Boolean) (SweepResult :type "HitResult Structure (by ref)"))
  (bind _widget (`self.Widget`))
  (bind _asbp_third_person_character (cast `/Game/ThirdPerson/Blueprints/BP_ThirdPersonCharacter` OtherActor))
  (if (`self.TerminalActive`)
    (set `/Game/ThirdPerson/Blueprints/BP_ThirdPersonCharacter.TerminalInRange` true _asbp_third_person_character :!label _label)
    (set `/Game/ThirdPerson/Blueprints/BP_ThirdPersonCharacter.Terminal` self _asbp_third_person_character)
    (bind _aswbp_pickup (cast `/Game/UI/WBP_Pickup` (`WidgetComponent.GetUserWidgetObject` _widget)))
    (`/Game/UI/WBP_Pickup.Set Text` _aswbp_pickup "POWER ON")
    (`SceneComponent.SetVisibility` _widget true false)
    (elif (`/Game/ThirdPerson/Blueprints/BP_ThirdPersonCharacter.CarryingPowerCell` _asbp_third_person_character)
      (set `/Game/ThirdPerson/Blueprints/BP_ThirdPersonCharacter.CarryingPowerCell` false _asbp_third_person_character)
      (set `self.TerminalActive` true)
      (`/Game/Blueprints/BP_AudioPlayer.PlaySound` (`self.ClickPlayer`))
      (goto _label)
      (else
        (`SceneComponent.SetVisibility` (`self.Widget`) true false)))))

(event `self.Sphere.OnComponentEndOverlap`
  (params (OverlappedComponent :type "PrimitiveComponent Object Reference") (OtherActor :type "Actor Object Reference") (OtherComp :type "PrimitiveComponent Object Reference") (OtherBodyIndex :type Integer))
  (bind _asbp_third_person_character (cast `/Game/ThirdPerson/Blueprints/BP_ThirdPersonCharacter` OtherActor))
  (set `/Game/ThirdPerson/Blueprints/BP_ThirdPersonCharacter.TerminalInRange` false _asbp_third_person_character)
  (`SceneComponent.SetVisibility` (`self.Widget`) false false))

(event `Complete`
  (`/Game/Blueprints/BP_AudioPlayer.PlaySound` (`self.SwitchPlayer`))
  (for _array_element (`self.LinkedLights`)
    (`SceneComponent.SetVisibility` (`Light.LightComponent` _array_element) true false))
  (for _array_element_2 (`self.LinkedSpawns`)
    (`/Game/Blueprints/BP_EnemySpawn.Spawn` _array_element_2))
  (`/Game/Blueprints/BP_AudioPlayer.PlaySound` (`self.MusicPlayer`)))

(fn `UserConstructionScript`)